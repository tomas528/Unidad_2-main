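; BP_Player is the player character Blueprint, handling Enhanced Input for movement, camera look, jump, run and melee-style montage attacks.
; BeginPlay adds IMC_Player; movement follows control yaw, and running toggles max walk speed.
; A second IA_Move handler also feeds controller yaw and pitch, duplicating the look logic.
; Attacks select a montage by AttackIndex and re-arm Canattack on completion, but the index increment is disconnected.
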(event `self.ReceiveBeginPlay`
  (bind _returnvalue (pcsubsystem `EnhancedInputLocalPlayerSubsystem` (`GameplayStatics.GetPlayerController` 0)))
  (`/Engine/EditorBlueprintResources/StandardMacros.IsValid` _returnvalue
    (:`Is Valid`
      (`EnhancedInputSubsystemInterface.AddMappingContext` _returnvalue "/Game/IA/IMC_Player.IMC_Player" 0 (struct)))))

(event `EnhancedInput|/Game/IA/IA_Move`
  (params (ActionValue :type "Vector2D Structure") (ElapsedSeconds :type "Float (double-precision)") (TriggeredSeconds :type "Float (double-precision)") (InputAction :type "InputAction Object Reference" :default "/Game/IA/IA_Move.IA_Move"))
  (bind (_returnvalue_roll _returnvalue_pitch _returnvalue_yaw) (`KismetMathLibrary.BreakRotator` (`self.GetControlRotation`)))
  (bind (_returnvalue_roll_2 _returnvalue_pitch_2 _returnvalue_yaw_2) (`KismetMathLibrary.BreakRotator` (`self.GetControlRotation`)))
  (:`Triggered`
    (`self.AddMovementInput` (`KismetMathLibrary.GetForwardVector` (`KismetMathLibrary.MakeRotator` 0.0 0.0 _returnvalue_yaw)) ActionValue_Y)
    (`self.AddMovementInput` (`KismetMathLibrary.GetRightVector` (`KismetMathLibrary.MakeRotator` 0.0 0.0 _returnvalue_yaw_2)) ActionValue_X)))

(event `EnhancedInput|/Game/IA/IA_Jump`
  (params (ActionValue :type Boolean) (ElapsedSeconds :type "Float (double-precision)") (TriggeredSeconds :type "Float (double-precision)") (InputAction :type "InputAction Object Reference" :default "/Game/IA/IA_Jump.IA_Jump"))
  (:`Triggered`
    (`self.Jump`)))

(event `EnhancedInput|/Game/IA/IA_Run`
  (params (ActionValue :type Boolean) (ElapsedSeconds :type "Float (double-precision)") (TriggeredSeconds :type "Float (double-precision)") (InputAction :type "InputAction Object Reference" :default "/Game/IA/IA_Run.IA_Run"))
  (bind _charactermovement (`self.CharacterMovement`))
  (:`Triggered`
    (set `CharacterMovementComponent.MaxWalkSpeed` 900.0 _charactermovement))
  (:`Canceled`
    (set `CharacterMovementComponent.MaxWalkSpeed` 400.0 _charactermovement :!label _label))
  (:`Completed`
    (goto _label)))

(event `EnhancedInput|/Game/IA/IA_Move`
  (params (ActionValue :type "Vector2D Structure") (ElapsedSeconds :type "Float (double-precision)") (TriggeredSeconds :type "Float (double-precision)") (InputAction :type "InputAction Object Reference" :default "/Game/IA/IA_Move.IA_Move"))
  (:`Triggered`
    (`self.AddControllerYawInput` ActionValue_X)
    (`self.AddControllerPitchInput` ActionValue_Y)))

(event `EnhancedInput|/Game/IA/IA_Look`
  (params (ActionValue :type "Vector2D Structure") (ElapsedSeconds :type "Float (double-precision)") (TriggeredSeconds :type "Float (double-precision)") (InputAction :type "InputAction Object Reference" :default "/Game/IA/IA_Look.IA_Look"))
  (:`Triggered`
    (`self.AddControllerYawInput` ActionValue_X)
    (`self.AddControllerPitchInput` ActionValue_Y)))

(event `EnhancedInput|/Game/IA/IA_Attack`
  (params (ActionValue :type Boolean) (ElapsedSeconds :type "Float (double-precision)") (TriggeredSeconds :type "Float (double-precision)") (InputAction :type "InputAction Object Reference" :default "/Game/IA/IA_Attack.IA_Attack"))
  (:`Triggered`
    (`self.Canattack`
      (:`then`
        (set `self.Canattack` false)
        (`|PlayMontage` (`self.Mesh`) (select `int` (`self.AttackIndex`) :`0` "/Game/BP_Player/Animations/01_Montage.01_Montage" :`1` "/Game/BP_Player/Animations/02_Montage.02_Montage" :`2` "/Game/BP_Player/Animations/03_Montage.03_Montage" :!type "AnimMontage Object Reference")
          (:`OnCompleted`
            (set `self.Canattack` true))))
      (:`else`))))

(fn `UserConstructionScript`)