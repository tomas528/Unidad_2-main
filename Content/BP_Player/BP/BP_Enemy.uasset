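; BP_Enemy is an enemy Blueprint that reacts to damage through two events, BPIDaño and BPIDamage.
; BPIDaño prints a hurt message, throttled by a DoOnce that resets after a short delay.
; BPIDamage subtracts a fixed amount from Vida, then always destroys the actor because its branch condition is constant true.
; The Vida zero-check is left unconnected, so the health printout never runs.
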(event `/Game/BP_Player/BP/BPI_Daño.BPI_Daño`
  (`/Engine/EditorBlueprintResources/StandardMacros.DoOnce` false :!label _label
    (:`Completed`
      (`KismetSystemLibrary.PrintString` "ahhh")
      (`KismetSystemLibrary.Delay` 0.5)
      (goto _label :!via `Reset`))))

(event `/Game/BP_Player/BP/BPI_Damage.BPI_Damage`
  (bind _output_get (set `self.Vida` (- (`self.Vida`) 10)))
  (if true
    (`self.K2_DestroyActor`)
    (else
      (`KismetSystemLibrary.PrintString` (`KismetStringLibrary.Conv_IntToString` (`self.Vida`))))))

(fn `UserConstructionScript`)