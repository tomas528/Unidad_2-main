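; BP_NPC is an NPC Blueprint with an unfinished dialogue interaction, and none of its logic runs.
; The BPI Interact graph holds only disconnected fragments: creating and caching a WB_Dialogue widget, casting to BP_Player, playing a sound and destroying the actor.
; Reads of the dialogue array and its index are unused.
; The construction script is empty.
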(fn `UserConstructionScript`)